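; Player pawn for the endless runner shooter, adding effects, game UI and achievement unlocks on top of its parent class.
; Firing spawns a muzzle flash at the gun's Muzzle socket and plays a gunshot before calling parent Fire.
; BeginPlay creates the game UI widget, and overlapping an AchivementTrigger increments and unlocks its achievement.
; Death enables mesh physics simulation, pauses the UI's Skills animation and plays a hit sound.
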(event Custom|PlayMuzzleFlashAndSound
  (bind _projectilespawnlocation (CallFunction|GetProjectileSpawnLocation))
  (Effects|SpawnEmitteratLocation "/Game/EndlessRunnerShooterTemplate/ParticleEffects/P_MuzzleFlash.P_MuzzleFlash" _projectilespawnlocation)
  (Audio|PlaySoundatLocation "/Game/EndlessRunnerShooterTemplate/Sounds/CUE_Gunshot.CUE_Gunshot" (Transformation|GetWorldLocation (Variables|Character|GetMesh)) "0, 0, 0" 1.0 1.0 0.0 0 0 0 0))

(event EventFire
  (CallFunction|PlayMuzzleFlashandSound)
  (|CallParentFunction))

(event EventBeginPlay
  (bind _returnvalue (UserInterface|CreateWidget "/Game/EndlessRunnerShooterTemplate/Widgets/BP_GameUI.BP_GameUI_C" 0 0))
  (UserInterface|Viewport|AddtoViewport _returnvalue 0)
  (Default|PlayAnima _returnvalue))

(event Collision|EventActorBeginOverlap
  (params (OtherActor :type Actor%20Object%20Reference))
  (Utilities|Casting|CastToAchivementTrigger OtherActor)
  (Variables|/Game/EndlessRunnerShooterTemplate/Widgets/BP_GameUI.BP_GameUI_C|SetAchivementToUnlock (stale EventBeginPlay _returnvalue) (+ (Variables|/Game/EndlessRunnerShooterTemplate/Widgets/BP_GameUI.BP_GameUI_C|GetAchivementToUnlock (stale EventBeginPlay _returnvalue)) 1))
  (Default|UnlockAchivement (stale EventBeginPlay _returnvalue)))

(event EventOnPlayerDied
  (Physics|SetSimulatePhysics (Variables|Character|GetMesh) true)
  (Class|UserWidget|PauseAnimation (stale EventBeginPlay _returnvalue) (Variables|/Game/EndlessRunnerShooterTemplate/Widgets/BP_GameUI.BP_GameUI_C|GetSkills (stale EventBeginPlay _returnvalue)))
  (Audio|PlaySound2D "/Game/Level/Hit_Cue.Hit_Cue" 1.0 1.0 0.0 0 0))

(fn ConstructionScript
  (|CallParentFunction))

(fn GetProjectileSpawnLocation
  (return (Transformation|GetSocketLocation (Variables|Default|GetGun) "Muzzle")))